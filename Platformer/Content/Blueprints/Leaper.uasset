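; Leaper is a sprite actor meant to move back and forth between two reference points, Pointa and Pointb.
; A timeline's alpha lerps the actor's location between them without sweep.
; Near either end of the alpha range, the sprite's world X scale is set positive or negative to mirror it.
; Nothing in the event graph triggers the timeline.
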(fn ConstructionScript)