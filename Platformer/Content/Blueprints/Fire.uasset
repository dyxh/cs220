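; Fire is a sprite actor scripted to travel between two referenced actors, Pointa and Pointb.
; A timeline alpha lerps between their locations and sets the actor's position without sweep.
; Near either end of the alpha range, the sprite's X scale flips sign to mirror it, with Y scale set to zero.
; Nothing in the graph calls the timeline to play.
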(fn ConstructionScript)